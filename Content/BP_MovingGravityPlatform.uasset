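; Moving platform that travels and rotates along the Track spline when a BP_ThirdPersonGravityCharacter enters its Box trigger.
; Construction and BeginPlay snap it to the spline start; each new entry alternates the Timeline between forward and reverse.
; Timeline output scales spline length to teleport the actor, applying local-space spline values as its world transform.
; An IsInside flag blocks retriggering until any actor overlap ends.
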(event OnComponentBeginOverlap(Box)
  (params (OverlappedComponent :type Primitive%20Component%20Object%20Reference) (OtherActor :type Actor%20Object%20Reference) (OtherComp :type Primitive%20Component%20Object%20Reference) (OtherBodyIndex :type Integer) (bFromSweep :type Boolean) (SweepResult :type Hit%20Result%20Structure%20%28by%20ref%29))
  (bind _track (Variables|Default|GetTrack))
  (Utilities|Casting|CastToBP_ThirdPersonGravityCharacter OtherActor)
  (if (not (Variables|Default|GetIsInside))
    (Variables|Default|SetIsInside true)
    (bind _output_get (Variables|Default|SetToggle (not (Variables|Default|GetToggle))))
    (if _output_get
      (bind _newtrack_0 (Timeline|Timeline Play)
        (:Update
          (Variables|Default|SetTrackPosition _newtrack_0)
          (Transformation|SetActorLocation (Spline|GetLocationatDistanceAlongSpline _track (* (Variables|Default|GetTrackPosition) (Spline|GetSplineLength (Variables|Default|GetTrack))) "Local") false true)
          (Transformation|SetActorRotation (Spline|GetRotationatDistanceAlongSpline _track (* (Variables|Default|GetTrackPosition) (Spline|GetSplineLength (Variables|Default|GetTrack))) "Local") true)))
      (else
        (Timeline|Timeline Reverse)))))

(event EventBeginPlay
  (bind _returnvalue (Math|Float|MakeLiteralFloat 0.0))
  (bind _track (Variables|Default|GetTrack))
  (Transformation|SetActorLocation (Spline|GetLocationatDistanceAlongSpline _track _returnvalue "Local") false false)
  (Transformation|SetActorRotation (Spline|GetRotationatDistanceAlongSpline _track _returnvalue "Local")))

(event EventTick
  (params (DeltaSeconds :type Float%20%28single-precision%29)))

(event Collision|EventActorEndOverlap
  (params (OtherActor :type Actor%20Object%20Reference))
  (Variables|Default|SetIsInside false))

(fn ConstructionScript
  (bind _returnvalue (Math|Float|MakeLiteralFloat 0.0))
  (bind _track (Variables|Default|GetTrack))
  (Transformation|SetActorLocation (Spline|GetLocationatDistanceAlongSpline _track _returnvalue "Local") false false)
  (Transformation|SetActorRotation (Spline|GetRotationatDistanceAlongSpline _track _returnvalue "Local")))