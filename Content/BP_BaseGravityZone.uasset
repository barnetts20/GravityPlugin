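; Base gravity zone actor that reports overlapping actors and supplies a gravity vector for its area.
; Overlap events feed the OnZone begin and end handlers, but on entry any Character that is not a BP_ThirdPersonGravityCharacter is dropped.
; GetGravityVector points along the actor's local down axis with BaseVector's magnitude, so rotating the zone turns gravity and the queried position has no effect.
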(event Collision|EventActorBeginOverlap
  (params (OtherActor :type Actor%20Object%20Reference))
  (bind _ascharacter (Utilities|Casting|CastToCharacter OtherActor)
    (:then
      (bind _asbp_third_person_gravity_character (Utilities|Casting|CastToBP_ThirdPersonGravityCharacter _ascharacter))
      (Class|GravityZone|OnZoneBeginOverlap _asbp_third_person_gravity_character))
    (:CastFailed
      (Class|GravityZone|OnZoneBeginOverlap OtherActor))))

(event Collision|EventActorEndOverlap
  (params (OtherActor :type Actor%20Object%20Reference))
  (Class|GravityZone|OnZoneEndOverlap OtherActor))

(fn ConstructionScript)

(fn GetGravityVector
  (params (InWorldPosition :type Vector%20%28by%20ref%29 :default "0, 0, 0"))
  (return (* (Transformation|GetActorUpVector) -1.0 (Math|Vector|VectorLength (Variables|Default|GetBaseVector)))))