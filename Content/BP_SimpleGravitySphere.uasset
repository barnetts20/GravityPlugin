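; BP_SimpleGravitySphere is a spherical gravity source that pulls toward the actor's location.
; GetGravityVector takes a world position and returns the normalized direction from it to the actor, scaled by the length of BaseVector.
; The pull has constant strength, with no distance falloff or range check.
; The event graph holds only disabled stubs, and the construction script just calls its parent.
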(event EventBeginPlay)

(event Collision|EventActorBeginOverlap
  (params (OtherActor :type Actor%20Object%20Reference))
  (|CallParentFunction OtherActor) ; This node is disabled and will not be called.\nDrag off pins to build functionality.
)

(event EventTick
  (params (DeltaSeconds :type Float%20%28single-precision%29)))

(fn ConstructionScript
  (|CallParentFunction))

(fn GetGravityVector
  (params (InWorldPosition :type Vector%20%28by%20ref%29 :default "0, 0, 0"))
  (return (* (Math|Vector|Normalize (- (Transformation|GetActorLocation) InWorldPosition)) (Math|Vector|VectorLength (Variables|Default|GetBaseVector)))))