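; Planet actor that supplies a radial gravity vector pointing toward its center.
; Construction and BeginPlay size a Planet sphere to PlanetRadius and an outer Sphere to that radius scaled by an influence ratio.
; GetGravityVector returns BaseVector's magnitude at or inside the radius, and outside scales it by radius over distance raised to a Falloff exponent.
; It also prints the resulting strength on each call.
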(event EventBeginPlay
  (Components|Sphere|SetSphereRadius (Variables|Default|GetSphere) (* (Variables|GravityZone|GetPlanet%20Radius) (Variables|GravityZone|GetInflueceRatio)) true)
  (Components|Sphere|SetSphereRadius (Variables|Default|GetPlanet) (Variables|GravityZone|GetPlanet%20Radius) true))

(event Collision|EventActorBeginOverlap
  (params (OtherActor :type Actor%20Object%20Reference))
  (|CallParentFunction OtherActor) ; This node is disabled and will not be called.\nDrag off pins to build functionality.
)

(event EventTick
  (params (DeltaSeconds :type Float%20%28single-precision%29)))

(fn ConstructionScript
  (|CallParentFunction)
  (Components|Sphere|SetSphereRadius (Variables|Default|GetSphere) (* (Variables|GravityZone|GetPlanet%20Radius) (Variables|GravityZone|GetInflueceRatio)) true)
  (Components|Sphere|SetSphereRadius (Variables|Default|GetPlanet) (Variables|GravityZone|GetPlanet%20Radius) true))

(fn GetGravityVector
  (params (InWorldPosition :type Vector%20%28by%20ref%29 :default "0, 0, 0"))
  (bind _returnvalue (Transformation|GetActorLocation))
  (bind _falloff (Variables|GravityZone|GetFalloff))
  (bind _basevector (Variables|Default|GetBaseVector))
  (bind _planet_radius (Variables|GravityZone|GetPlanet%20Radius))
  (bind _returnvalue_2 (Math|Vector|VectorLength _basevector))
  (bind _returnvalue_3 (- _returnvalue InWorldPosition))
  (bind _returnvalue_4 (Math|Vector|Normalize _returnvalue_3))
  (bind _returnvalue_5 (Math|Vector|VectorLength _returnvalue_3))
  (bind _returnvalue_6 (* _returnvalue_4 _returnvalue_2))
  (bind _returnvalue_7 (/ _planet_radius _returnvalue_5))
  (bind _returnvalue_8 (Math|Float|Power _returnvalue_7 _falloff))
  (bind _returnvalue_9 (* _returnvalue_6 _returnvalue_8))
  (if (> _returnvalue_5 _planet_radius)
    (Development|PrintString (Utilities|String|ToString(Float) (Math|Vector|VectorLength _returnvalue_9)))
    (return _returnvalue_9)
    (else
      (Development|PrintString (Utilities|String|ToString(Float) (Math|Vector|VectorLength _returnvalue_6)))
      (return _returnvalue_6))))